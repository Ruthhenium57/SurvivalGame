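; Flashlight prop Blueprint with a static mesh and a spot light whose on/off state and brightness are configured per instance.
; The construction script creates a dynamic material instance on the mesh's second material slot.
; A switch variable then sets both the emissive parameter and spot light intensity, scaled from one intensity value, or zeroes both when off.
; The event graph holds only disabled default events, so nothing changes at runtime.
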(event EventBeginPlay)

(event Collision|EventActorBeginOverlap
  (params (OtherActor :type Actor%20Object%20Reference)))

(event EventTick
  (params (DeltaSeconds :type Float%20%28single-precision%29)))

(fn ConstructionScript
  (bind _lightintensity (Variables|Default|GetLightIntensity))
  (bind _spotlight (Variables|Default|GetSpotLight))
  (bind _returnvalue (Rendering|Material|CreateDynamicMaterialInstance (Variables|Default|GetStaticMesh) 1 "/Game/SurvivalProps/Materials/Flashlight_mat.Flashlight_mat" :!class /Script/Engine.PrimitiveComponent))
  (Variables|Default|SetDMI _returnvalue)
  (if (Variables|Default|GetLight%20Switch)
    (Rendering|Material|SetScalarParameterValue (Variables|Default|GetDMI) "Emissive" (* _lightintensity 1e+02) :!class /Script/Engine.MaterialInstanceDynamic)
    (Rendering|Components|Light|SetIntensity _spotlight (* _lightintensity 2.5e+03))
    (else
      (Rendering|Material|SetScalarParameterValue (Variables|Default|GetDMI) "Emissive" 0.0 :!class /Script/Engine.MaterialInstanceDynamic)
      (Rendering|Components|Light|SetIntensity _spotlight 0.0))))